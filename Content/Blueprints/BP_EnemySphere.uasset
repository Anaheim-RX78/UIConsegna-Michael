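; BP_EnemySphere is an enemy that chases the first-person player and sends the game back to the main menu on touch.
; From BeginPlay it runs a self-restarting AIMoveTo loop toward the player, retrying after a short delay on success or failure.
; Overlapping projectiles lower its Health, update the health bar in its widget component, and destroy the enemy when Health runs out.
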(event EventBeginPlay
  (Utilities|FlowControl|Sequence
    (:then_0
      (bind _returnvalue (Actor|GetActorOfClass "/Game/FirstPerson/Blueprints/BP_FirstPersonCharacter.BP_FirstPersonCharacter_C"))
      (AI|AIMoveTo self "0, 0, 0" _returnvalue 5.0 false :!label _label
        (:OnSuccess
          (Utilities|FlowControl|Delay 0.4)
          (goto _label))
        (:OnFail
          (Utilities|FlowControl|Delay 1.0)
          (goto _label))))
    (:then_1
      (bind _output_get (Variables|Default|SetHealth 1.0))
      (bind _asbp_health_bar (Utilities|Casting|CastToBP_HealthBar (UserInterface|GetWidget (Variables|Default|GetWidget))))
      (Progress|SetPercent (Variables|/Game/FirstPerson/Blueprints/BP_HealthBar.BP_HealthBar_C|GetProgressBar_23 _asbp_health_bar) _output_get))))

(event EventTick
  (params (DeltaSeconds :type Float%20%28single-precision%29)))

(event Collision|EventActorBeginOverlap
  (params (OtherActor :type Actor%20Object%20Reference))
  (Utilities|Casting|CastToBP_FirstPersonCharacter OtherActor
    (:then
      (Game|OpenLevel(byObjectReference) "/Game/FirstPerson/Maps/MainMenu.MainMenu"))
    (:CastFailed
      (Utilities|Casting|CastToBP_FirstPersonProjectile OtherActor)
      (bind _output_get (Variables|Default|SetHealth (- (Variables|Default|GetHealth) 0.1)))
      (bind _asbp_health_bar (Utilities|Casting|CastToBP_HealthBar (UserInterface|GetWidget (Variables|Default|GetWidget))))
      (Progress|SetPercent (Variables|/Game/FirstPerson/Blueprints/BP_HealthBar.BP_HealthBar_C|GetProgressBar_23 _asbp_health_bar) _output_get)
      (if (<= (Variables|Default|GetHealth) 0.0)
        (Actor|DestroyActor)))))

(fn ConstructionScript)